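; Game mode that runs the round timer and moves play between DemoLevel and DemoLevel2.
; BeginPlay adds the timer widget and, on DemoLevel, zeroes the timer and the game instance's time, lives and points.
; Tick uses Delay as a one-second throttle, counting MyTimer until IsRoundFinished, then MyBeginTimer up to a short threshold.
; It then opens DemoLevel2 from DemoLevel, otherwise resets those stats and returns to DemoLevel.
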(event `self.ReceiveBeginPlay`
  (bind _returnvalue (`|CreateWidget` "/Game/FrameWork/TimerWidget_BP.TimerWidget_BP_C"))
  (`UserWidget.AddToViewport` _returnvalue 1)
  (bind _returnvalue_2 (`GameplayStatics.GetCurrentLevelName` true))
  (if (`KismetStringLibrary.EqualEqual_StrStr` _returnvalue_2 "DemoLevel")
    (set `self.myTimer` 0)
    (bind _asmy_game_instance_tpunreal_bp (cast `/Game/MyGameInstanceTPUnreal_BP` (`GameplayStatics.GetGameInstance`)))
    (set `GameInstanceTPUnreal.currentTime` 0 _asmy_game_instance_tpunreal_bp)
    (set `GameInstanceTPUnreal.playersLifes` 0 _asmy_game_instance_tpunreal_bp)
    (set `GameInstanceTPUnreal.points` 0 _asmy_game_instance_tpunreal_bp)))

(event `self.ReceiveTick`
  (params (DeltaSeconds :type "Float (single-precision)"))
  (if (`self.IsRoundFinished`)
    (`KismetSystemLibrary.Delay` 1.0)
    (bind _result (`/Engine/EditorBlueprintResources/StandardMacros.IncrementInt` (`self.myBeginTimer`))
      (:`  `
        (bind _output_get (set `self.myBeginTimer` _result))
        (if (>= _output_get 5)
          (bind _returnvalue (`GameplayStatics.GetCurrentLevelName` true))
          (if (`KismetStringLibrary.EqualEqual_StrStr` _returnvalue "DemoLevel")
            (`GameplayStatics.OpenLevel` "DemoLevel2")
            (else
              (bind _asmy_game_instance_tpunreal_bp (cast `/Game/MyGameInstanceTPUnreal_BP` (`GameplayStatics.GetGameInstance`)))
              (set `GameInstanceTPUnreal.currentTime` 0 _asmy_game_instance_tpunreal_bp)
              (set `GameInstanceTPUnreal.playersLifes` 0 _asmy_game_instance_tpunreal_bp)
              (set `GameInstanceTPUnreal.points` 0 _asmy_game_instance_tpunreal_bp)
              (`GameplayStatics.OpenLevel` "DemoLevel"))))))
    (else
      (`KismetSystemLibrary.Delay` 1.0)
      (bind _result_2 (`/Engine/EditorBlueprintResources/StandardMacros.IncrementInt` (`self.myTimer`))
        (:`  `
          (set `self.myTimer` _result_2))))))

(fn `UserConstructionScript`)